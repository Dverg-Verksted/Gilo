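; Patrol bot pawn for the horror game that runs BT_PatrolBot and senses player characters through AI perception.
; On possession it starts the behavior tree and copies its walk and run speeds into the blackboard.
; Perception updates set the sensed player as the enemy and store the stimulus location as the target.
; Losing the player clears the enemy but still writes that stimulus location to the target key.
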(event `self.ReceivePossessed`
  (params (NewController :type "Controller Object Reference"))
  (`self.Initialize` NewController))

(event `self.PerceptionComponent.OnTargetPerceptionUpdated`
  (params (Actor :type "Actor Object Reference") (Stimulus :type "AIStimulus Structure"))
  (`self.UpdateEnemy` Actor Stimulus))

(fn `Initialize`
  (params (Controller :type "Object Object Reference"))
  (bind _asaicontroller (cast `AIController` Controller))
  (`AIController.RunBehaviorTree` _asaicontroller "/Game/HorrorGame/Core/AI/BehaviorTree/BT_PatrolBot.BT_PatrolBot")
  (bind _returnvalue (`AIBlueprintHelperLibrary.GetBlackboard` _asaicontroller))
  (`BlackboardComponent.SetValueAsFloat` _returnvalue (`self.WalkSpeedKey`) (`self.WalkSpeed`))
  (`BlackboardComponent.SetValueAsFloat` _returnvalue (`self.RunSpeedKey`) (`self.RunSpeed`)))

(fn `UpdateEnemy`
  (params (EnemyActor :type "Object Object Reference") (AIStimulus :type "AIStimulus Structure (by ref)"))
  (bind (_age _expirationage _strength _stimuluslocation _receiverlocation _tag _bsuccessfullysensed) (break `AIStimulus` AIStimulus))
  (bind _asaicontroller (cast `AIController` (`self.GetController`)))
  (bind _asplayer_character_base (cast `PlayerCharacterBase` EnemyActor))
  (if _bsuccessfullysensed
    (bind _returnvalue (`AIBlueprintHelperLibrary.GetBlackboard` _asaicontroller))
    (`BlackboardComponent.SetValueAsObject` _returnvalue (`self.EnemyKey`) _asplayer_character_base)
    (`BlackboardComponent.SetValueAsVector` _returnvalue (`self.TargetLocationKey`) _stimuluslocation)
    (else
      (`BlackboardComponent.SetValueAsObject` _returnvalue (`self.EnemyKey`) null)
      (`BlackboardComponent.SetValueAsVector` _returnvalue (`self.TargetLocationKey`) _stimuluslocation))))

(fn `UserConstructionScript`)