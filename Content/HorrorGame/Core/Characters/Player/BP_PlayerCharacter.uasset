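; Player character Blueprint for the horror game, handling damage and stamina audio and telling bots when the player perceives them.
; A damage cue plays on hit, and stamina changes drive the breathing sound's fatigue parameter.
; AI Perception updates toggle bots in a tracked array, calling CharacterIsSee on their AI controllers, without reading the stimulus.
; GetHUD returns the game HUD through the player controller.
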(event `self.ReceiveAnyDamage`
  (params (Damage :type "Float (single-precision)") (DamageType :type "DamageType Object Reference") (InstigatedBy :type "Controller Object Reference") (DamageCauser :type "Actor Object Reference"))
  (`GameplayStatics.PlaySound2D` "/Game/HorrorGame/Sounds/SFX/Player/A_PlayerDamage_Cue.A_PlayerDamage_Cue" 1.0 1.0 0.0 null null))

(event `self.PlayerSprintComponent.OnStaminaChanged`
  (params (Stamina :type "Float (single-precision)") (Fatigue :type "Float (single-precision)"))
  (`AudioParameterControllerInterface.SetFloatParameter` (`self.Audio_SprintBreath`) "Fatigue" Fatigue))

(event `self.AIPerception.OnTargetPerceptionUpdated`
  (params (Actor :type "Actor Object Reference") (Stimulus :type "AIStimulus Structure"))
  (bind _actor (`self.Actor`))
  (bind _index (`self.index`))
  (bind _asbp_bot_base (cast `/Game/HorrorGame/Core/Bot/BP_BotBase` Actor))
  (bind _returnvalue (`KismetArrayLibrary.Array_Find` _actor _asbp_bot_base))
  (if (== _returnvalue -1)
    (`KismetArrayLibrary.Array_Insert` _actor _asbp_bot_base _index)
    (`/Engine/EditorBlueprintResources/StandardMacros.IncrementInt` _index
      (:`  `
        (for _array_element _actor
          (bind _asbp_aicontroller_base (cast `/Game/HorrorGame/Core/Bot/BP_AIControllerBase` (`AIBlueprintHelperLibrary.GetAIController` _array_element)))
          (`AIControllerBase.CharacterIsSee` _asbp_aicontroller_base true))))
    (else
      (bind _asbp_aicontroller_base_2 (cast `/Game/HorrorGame/Core/Bot/BP_AIControllerBase` (`AIBlueprintHelperLibrary.GetAIController` _asbp_bot_base)))
      (`AIControllerBase.CharacterIsSee` _asbp_aicontroller_base_2 false)
      (`KismetArrayLibrary.Array_Remove` _actor _returnvalue)
      (`/Engine/EditorBlueprintResources/StandardMacros.DecrementInt` _index))))

(fn `GetHUD`
  (returns (GameHUD :type "/Game/HorrorGame/Core/UI/HUD/BP_GameHUD Object Reference"))
  (bind _asplayer_controller (cast `PlayerController` (`self.GetController`))
    (:`then`
      (bind _asbp_game_hud (cast `/Game/HorrorGame/Core/UI/HUD/BP_GameHUD` (`PlayerController.GetHUD` _asplayer_controller))))
    (:`CastFailed`
      _))
  (return _asbp_game_hud))

(fn `UserConstructionScript`)