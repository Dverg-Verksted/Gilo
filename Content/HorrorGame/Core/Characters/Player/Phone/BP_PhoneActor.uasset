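; BP_PhoneActor is the player's phone in the horror game, with a mesh that can be shown or hidden and a spotlight flashlight that toggles.
; Showing the phone reapplies the stored flashlight state after visibility propagates to the mesh's children.
; On BeginPlay it finds the player character's BP_PhoneMessagerComponent and binds to its new-message event.
; New messages play a notification sound at the phone's location.
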(event `self.ReceiveBeginPlay`
  ;[1 0.4275 0] Initialize
  (`self.Initialize`))

(event `ShowPhone`
  ;[1 1 1] Show Phone
  (`SceneComponent.SetVisibility` (`self.PhoneMesh`) true true)
  (`self.SetFlashLightVisible` (`self.FlashLightVisible`)))

(event `HidePhone`
  ;[1 1 1] Hide Phone
  (`SceneComponent.SetVisibility` (`self.PhoneMesh`) false true))

(event `ToggleFlashLight`
  ;[1 1 1] Toggle FlashLight
  (`self.SetFlashLightVisible` (not (`self.FlashLightVisible`))))

(event `OnNewMessage`
  (params (Message :type "/Game/HorrorGame/Core/UI/Player/Phone/BP_PhoneMessage Object Reference"))
  ;[1 1 1] On New Message
  (`GameplayStatics.PlaySoundAtLocation` "/Game/HorrorGame/Sounds/SFX/Player/A_PhoneMessage_Cue.A_PhoneMessage_Cue" (`self.K2_GetActorLocation`) (`self.K2_GetActorRotation`) 1.0 1.0 0.0 null null self null))

(fn `Initialize`
  (bind _returnvalue (`GameplayStatics.GetPlayerCharacter` 0))
  (bind _returnvalue_2 (`self.GetComponentByClass` _returnvalue "/Game/HorrorGame/Core/UI/Player/Phone/BP_PhoneMessagerComponent.BP_PhoneMessagerComponent_C"))
  (`/Engine/EditorBlueprintResources/StandardMacros.IsValid` _returnvalue
    (:`Is Valid`
      (`/Engine/EditorBlueprintResources/StandardMacros.IsValid` _returnvalue_2
        (:`Is Valid`
          (bind _output_get (set `self.MessagerComponent` _returnvalue_2))
          (add `/Game/HorrorGame/Core/UI/Player/Phone/BP_PhoneMessagerComponent.OnNewMessage` _output_get (`|CreateDelegate` :!event `OnNewMessage`)))))))

(fn `SetFlashLightVisible`
  (params (Visible :type Boolean))
  (`SceneComponent.SetVisibility` (`self.SpotLight`) Visible true)
  (set `self.FlashLightVisible` Visible))

(fn `UserConstructionScript`)