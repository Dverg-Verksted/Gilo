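; BP_PhoneManagerComponent is an actor component that controls the player's smartphone in the horror game.
; On BeginPlay it looks for a BP_PhoneActor among its owner's child actors, caches it and starts it hidden.
; Enhanced Input actions toggle the phone's visibility and, only while it is showing, its flashlight.
; The component tracks the shown state and delegates the actual behavior to the phone actor.
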(event `self.ReceiveBeginPlay`
  ;[1 0.6255 0] Initialize
  (`self.Initialize`))

(event `EnhancedInput|/Game/HorrorGame/Core/Characters/Player/Input/IA_SmartPhone`
  (params (ActionValue :type Boolean) (ElapsedSeconds :type "Float (double-precision)") (TriggeredSeconds :type "Float (double-precision)") (InputAction :type "InputAction Object Reference" :default "/Game/HorrorGame/Core/Characters/Player/Input/IA_SmartPhone.IA_SmartPhone"))
  ;[1 1 1] Toggle Phone
  (:`Triggered`
    (if (`self.PhoneShowing`)
      (`self.HidePhone`)
      (else
        (`self.ShowPhone`)))))

(event `ShowPhone`
  ;[1 1 1] Show Phone
  (`/Engine/EditorBlueprintResources/StandardMacros.IsValid` (`self.PhoneActor`)
    (:`Is Valid`
      (`/Game/HorrorGame/Core/Characters/Player/Phone/BP_PhoneActor.ShowPhone` (`self.PhoneActor`))
      (set `self.PhoneShowing` true))))

(event `HidePhone`
  ;[1 1 1] Hide Phone
  (`/Engine/EditorBlueprintResources/StandardMacros.IsValid` (`self.PhoneActor`)
    (:`Is Valid`
      (`/Game/HorrorGame/Core/Characters/Player/Phone/BP_PhoneActor.HidePhone` (`self.PhoneActor`))
      (set `self.PhoneShowing` false))))

(event `EnhancedInput|/Game/HorrorGame/Core/Characters/Player/Input/IA_FlashLight`
  (params (ActionValue :type Boolean) (ElapsedSeconds :type "Float (double-precision)") (TriggeredSeconds :type "Float (double-precision)") (InputAction :type "InputAction Object Reference" :default "/Game/HorrorGame/Core/Characters/Player/Input/IA_FlashLight.IA_FlashLight"))
  (bind _phoneactor (`self.PhoneActor`))
  ;[1 1 1] Toggle Flashlight
  (:`Triggered`
    (if (`self.PhoneShowing`)
      (`/Engine/EditorBlueprintResources/StandardMacros.IsValid` _phoneactor
        (:`Is Valid`
          (`/Game/HorrorGame/Core/Characters/Player/Phone/BP_PhoneActor.ToggleFlashLight` _phoneactor))))))

(fn `GetPhoneActor`
  (returns (Success :type Boolean))
  (for _array_element (`Actor.GetAllChildActors` (`self.GetOwner`) true)
    (bind _asbp_phone_actor (cast `/Game/HorrorGame/Core/Characters/Player/Phone/BP_PhoneActor` _array_element))
    (set `self.PhoneActor` _asbp_phone_actor)
    (return true))
  (return false))

(fn `Initialize`
  (bind _success (`self.GetPhoneActor`))
  (if _success
    (`self.HidePhone`)))