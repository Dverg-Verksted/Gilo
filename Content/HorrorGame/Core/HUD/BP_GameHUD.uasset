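; BP_GameHUD is the horror game's HUD, which creates the player's crosshair and the CommonUI base widget on BeginPlay.
; PushPrompt and PushMenu forward requests to that base widget, which manages the active menus.
; ToggleGameMenu pushes UI_GameMenu or deactivates it if it is the active menu, switching input mode, mouse cursor and game pause to match.
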(event `self.ReceiveBeginPlay`
  (`self.AddDefaultWidgets` (`GameplayStatics.GetPlayerController` 0)))

(fn `AddDefaultWidgets`
  (params (OwningPlayer :type "PlayerController Object Reference"))
  (locals (player :type "PlayerController Object Reference"))
  (set `local.player` OwningPlayer)
  (`|ExecutionSequence`
    (:`then_0`
      ;[1 1 1] Crosshair
      (bind _returnvalue (`|CreateWidget` "/Game/HorrorGame/Core/UI/Player/WBP_Crosshair.WBP_Crosshair_C" (`local.player`)))
      (bind _output_get (set `self.CrosshairWidget` _returnvalue))
      (`UserWidget.AddToViewport` _output_get 0))
    (:`then_1`
      ;[1 1 1] CommonUI Base Widget
      (bind _returnvalue_2 (`|CreateWidget` "/Game/HorrorGame/Core/UI/UI_Base.UI_Base_C" (`local.player`)))
      (bind _output_get_2 (set `self.BaseUI` _returnvalue_2))
      (`UserWidget.AddToViewport` _output_get_2 0))))

(fn `PushMenu`
  (params (MenuClass :type "CommonActivatableWidget Class Reference"))
  (returns (MenuWidget :type "CommonActivatableWidget Object Reference"))
  (`/Engine/EditorBlueprintResources/StandardMacros.IsValid` (`self.BaseUI`)
    (:`Is Valid`
      (bind _menuwidget (`/Game/HorrorGame/Core/UI/UI_Base.PushMenu` (`self.BaseUI`) MenuClass))
      (return _menuwidget))))

(fn `PushPrompt`
  (params (Caption :type Text) (ConfirmCaption :type Text) (CancelCaption :type Text))
  (returns (PromptWidget :type "/Game/HorrorGame/Core/UI/UI_Generic_Prompt Object Reference"))
  (bind _promptwidget (`/Game/HorrorGame/Core/UI/UI_Base.PushPrompt` (`self.BaseUI`) Caption ConfirmCaption CancelCaption))
  (return _promptwidget))

(fn `ToggleGameMenu`
  (bind _returnvalue (`self.GetOwningPlayerController`))
  (bind _returnvalue_2 (`self.GetOwningPlayerController`))
  (bind (_success _activewidget) (`/Game/HorrorGame/Core/UI/UI_Base.IsAnyMenuActivated` (`self.BaseUI`)))
  (if _success
    (bind _asui_game_menu (cast `/Game/HorrorGame/Core/UI/UI_GameMenu` _activewidget))
    (`CommonActivatableWidget.DeactivateWidget` _asui_game_menu)
    (`WidgetBlueprintLibrary.SetInputMode_GameOnly` _returnvalue_2)
    (set `PlayerController.bShowMouseCursor` false _returnvalue_2)
    ;[1 1 1] Unpause game
    (`GameplayStatics.SetGamePaused` false)
    (else
      (`self.PushMenu` "/Game/HorrorGame/Core/UI/UI_GameMenu.UI_GameMenu_C")
      (`WidgetBlueprintLibrary.SetInputMode_UIOnlyEx` _returnvalue (`self.BaseUI`))
      (set `PlayerController.bShowMouseCursor` true _returnvalue)
      ;[1 1 1] Pause Game
      (`GameplayStatics.SetGamePaused` true))))

(fn `UserConstructionScript`)