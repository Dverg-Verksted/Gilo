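; BP_PhoneMessageTrigger is an overlap trigger that delivers a text message to the player's in-game phone.
; When an actor overlaps it while armed, it disarms, casts to PlayerCharacterBase and passes a timestamped message with configurable text and sender to the character's BP_PhoneMessagerComponent.
; Unless set to one-shot, it rearms after a cooldown delay.
; The disarm precedes the cast, so a non-player overlap also disarms it without rearming.
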(event `self.ReceiveActorBeginOverlap`
  (params (OtherActor :type "Actor Object Reference"))
  (if (`self.AddMessage`)
    (set `self.AddMessage` false)
    (bind _asplayer_character_base (cast `PlayerCharacterBase` OtherActor))
    (`/Game/HorrorGame/Core/UI/Player/Phone/BP_PhoneMessagerComponent.AddNewMessage` (`self.GetComponentByClass` _asplayer_character_base "/Game/HorrorGame/Core/UI/Player/Phone/BP_PhoneMessagerComponent.BP_PhoneMessagerComponent_C") (make `/Game/HorrorGame/Core/UI/Player/Phone/PhoneMessage` (`self.MessageText`) (`KismetMathLibrary.Now`) (`self.MessageSender`)))
    (if (not (`self.OneShot`))
      ;[1 1 1] Can add message after cooldown
      (`KismetSystemLibrary.Delay` (`self.CoolDown`))
      (set `self.AddMessage` true))))

(fn `UserConstructionScript`)