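; Interactable object Blueprint that shows an on-screen widget while a player hovers over it.
; On hover begin it creates the widget for that PlayerController, passing in short and long action values, and adds it to the viewport.
; Hover end and EndPlay both call ClearWidget, which validates the widget and removes it from its parent.
; CanBeGrabbed always returns false, marking the object as not grabbable.
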(event `self.OnHoverBegin`
  (params (PlayerController :type "PlayerController Object Reference") (Hit :type "HitResult Structure (by ref)"))
  (bind _returnvalue (`|CreateWidget` "/Game/HorrorGame/Core/Interactables/UserWidget.UserWidget_C" PlayerController (`self.ShortAction`) (`self.LongAction`)))
  (bind _output_get (set `self.Widget` _returnvalue))
  (`UserWidget.AddToViewport` _output_get 0))

(event `self.OnHoverEnd`
  (params (PlayerController :type "PlayerController Object Reference"))
  (`self.ClearWidget`))

(event `self.ReceiveEndPlay`
  (params (EndPlayReason :type "EEndPlayReason Enum" :default "Destroyed"))
  (`self.ClearWidget`))

(fn `CanBeGrabbed`
  (returns (CanBeGrabbed :type Boolean) (ComponentToGrab :type "PrimitiveComponent Object Reference"))
  (return false null))

(fn `ClearWidget`
  (`/Engine/EditorBlueprintResources/StandardMacros.IsValid` "/Game/HorrorGame/Core/Interactables/UserWidget.UserWidget"
    (:`Is Valid`
      (`Widget.RemoveFromParent` (`self.Widget`)))))