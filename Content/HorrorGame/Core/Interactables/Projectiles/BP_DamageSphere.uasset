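; BP_DamageSphere is an overlap damage volume that can be switched on and off, kept with the game's projectile interactables.
; ToggleDamageSphere switches query collision, sets the instigator and ignore list, and clears the record of damaged actors.
; While enabled, each overlapping actor not ignored takes damage once per activation, with the sphere's owner as causer, and fires OnActorDamaged.
; An optional one-shot mode disables the sphere after the first hit.
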(event `self.ReceiveBeginPlay`
  ;[1 0.4705 0] Initialize
  (`self.Initialize`))

(event `self.ReceiveActorBeginOverlap`
  (params (OtherActor :type "Actor Object Reference"))
  (`self.DamageActor` OtherActor))

(fn `DamageActor`
  (params (Actor :type "Actor Object Reference (by ref)"))
  (if (`self.DamageEnabled`)
    ;[1 1 1] Check is actor ignored
    (if (not (`KismetArrayLibrary.Array_Contains` (`self.ActorsToIgnore`) (`local.Actor`)))
      ;[1 1 1] Check is actor already damaged
      (if (not (`KismetArrayLibrary.Array_Contains` (`self.DamagedActors`) (`local.Actor`)))
        ;[1 1 1] Ignore actor in future
        (`KismetArrayLibrary.Array_Add` (`self.DamagedActors`) (`local.Actor`))
        ;[1 1 1] Apply Damage
        (`GameplayStatics.ApplyDamage` (`local.Actor`) (`self.DamageAmount`) (`self.GetDamageInstigator`) (`self.GetOwner`) (`self.DamageType`))
        (`self.OnActorDamaged` (`local.Actor`))
        ;[1 1 1] Disable if one shot mode
        (if (`self.OneShot`)
          (`self.ToggleDamageSphere` false null (`|MakeArray`)))))))

(fn `GetDamageInstigator`
  (returns (Instigator :type "Controller Object Reference"))
  (return (`self.DamageInstigator`)))

(fn `Initialize`
  (`PrimitiveComponent.SetCollisionProfileName` (`self.DamageSphere`) (`.Name` (break `CollisionProfileName` (`self.CollisionProfile`))) true))

(fn `ToggleDamageSphere`
  (params (Enabled :type Boolean) (Instigator :type "Controller Object Reference") (IgnoreActors :type "Array of Actor Object Reference"))
  (bind _output_get (set `self.DamageEnabled` Enabled))
  (`KismetArrayLibrary.Array_Clear` (`self.DamagedActors`))
  (if _output_get
    (`PrimitiveComponent.SetCollisionEnabled` (`self.DamageSphere`) "QueryOnly")
    (set `self.DamageInstigator` (`local.Instigator`))
    (set `self.ActorsToIgnore` (`local.IgnoreActors`))
    (else
      (`PrimitiveComponent.SetCollisionEnabled` (`self.DamageSphere`) "NoCollision")
      (set `self.DamageInstigator` null)
      (`KismetArrayLibrary.Array_Clear` (`self.ActorsToIgnore`)))))

(fn `UserConstructionScript`)