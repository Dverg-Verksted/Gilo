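; BP_HideCabinet is an interactable cabinet the player can climb into and out of to hide.
; Enter and exit events each open all doors, wait briefly, and blend the camera to the cabinet or back to the pawn.
; Timelines then lerp the pawn's transform to an inner spot, or from it to an exit spot, both composed relative to the cabinet, and close the doors when finished.
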(event `self.OnPlayerEnter`
  (params (PlayerController :type "PlayerController Object Reference"))
  (bind _returnvalue (`Controller.K2_GetPawn` PlayerController))
  (`self.OpenAllDoors`)
  (`KismetSystemLibrary.Delay` 0.6)
  (set `self.PlayerEnterTransform` (`self.GetTransform` _returnvalue))
  (`PlayerController.SetViewTargetWithBlend` PlayerController self 0.6 "VTBlend_Linear" 0.0 false)
  (bind (_direction _alpha) (`Timeline|PlayerEnterTimeline` :!via `PlayFromStart`)
    (:`Update`
      (`self.K2_SetActorTransform` _returnvalue (`KismetMathLibrary.TLerp` (`self.PlayerEnterTransform`) (`KismetMathLibrary.ComposeTransforms` (`self.GetTransform`) (`self.PlayerInnerTransform`)) _alpha) false false))
    (:`Finished`
      (`self.CloseAllDoors`))))

(event `self.OnPlayerExit`
  (params (PlayerController :type "PlayerController Object Reference"))
  (bind _returnvalue (`Controller.K2_GetPawn` PlayerController))
  (`self.OpenAllDoors`)
  (`KismetSystemLibrary.Delay` 0.3)
  (`PlayerController.SetViewTargetWithBlend` PlayerController _returnvalue 0.8 "VTBlend_Linear" 0.0 false)
  (bind (_direction _alpha) (`Timeline|PlayerExitTimeline` :!via `PlayFromStart`)
    (:`Update`
      (`self.K2_SetActorTransform` _returnvalue (`KismetMathLibrary.ComposeTransforms` (`self.GetTransform`) (`KismetMathLibrary.TLerp` (`self.PlayerInnerTransform`) (`self.PlayerExitTransform`) _alpha)) false false))
    (:`Finished`
      (`self.CloseAllDoors`))))

(fn `UserConstructionScript`)